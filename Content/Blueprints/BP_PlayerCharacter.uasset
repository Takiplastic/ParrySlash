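; Player character Blueprint whose event graph holds only debug input for checking combo gameplay tags.
; Key 1 prints the gameplay tags owned by the Ability System, or a notice when there are none.
; Key 2 prints a deletion message and removes the owned tags as non-replicated loose tags.
; BeginPlay, overlap, Tick and the construction script contain no logic.
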(event `self.ReceiveTick`
  (params (DeltaSeconds :type "Float (single-precision)")))

(event `Key|One`
  (params (Key :type "Key Structure"))
  (bind _returnvalue (`BlueprintGameplayTagLibrary.GetOwnedGameplayTags` (`self.AbilitySystem`)))
  ; コンボデバッグ用(タグ確認)
  (:`Pressed`
    (`KismetSystemLibrary.PrintString` (select `bool` (> (`BlueprintGameplayTagLibrary.GetNumGameplayTagsInContainer` _returnvalue) 0) :`false` "Do not have Tag" :`true` (`BlueprintGameplayTagLibrary.GetDebugStringFromGameplayTagContainer` _returnvalue)))))

(event `Key|Two`
  (params (Key :type "Key Structure"))
  (:`Pressed`
    (`KismetSystemLibrary.PrintString` "GameplayTags Deleted")
    (for _array_element (`|MakeArray` (`BlueprintGameplayTagLibrary.GetOwnedGameplayTags` (`self.AbilitySystem`)))
      (`AbilitySystemBlueprintLibrary.RemoveLooseGameplayTags` null _array_element))))

(fn `UserConstructionScript`)